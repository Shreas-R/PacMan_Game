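; Base pickup actor for collectible dots and power pickups, with behavior chosen by a PickupType value.
; When the first player character overlaps PickupRadius, it messages the GameState to raise the collected count, plays a type-specific 2D sound, then destroys itself.
; Power pickups also send the GameState a power-pickup message, and the construction script sets their mesh scale to set them apart.
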(event `self.PickupRadius.OnComponentBeginOverlap`
  (params (OverlappedComponent :type "PrimitiveComponent Object Reference") (OtherActor :type "Actor Object Reference") (OtherComp :type "PrimitiveComponent Object Reference") (OtherBodyIndex :type Integer) (bFromSweep :type Boolean) (SweepResult :type "HitResult Structure (by ref)"))
  (if (== (`GameplayStatics.GetPlayerCharacter` 0) OtherActor)
    (message `/Game/Blueprints/GameFramework/Interfaces/BPI_GameFramework.IncreaseCollectedCount` (`GameplayStatics.GetGameState`))
    (`self.PlaySound`)
    (switch `/Game/Blueprints/Data/e_PickupType` (`self.PickupType`)
      (:`NewEnumerator0`
        _)
      (:`NewEnumerator1`
        (message `/Game/Blueprints/GameFramework/Interfaces/BPI_GameFramework.CollectedPowerPickup` (`GameplayStatics.GetGameState`))))
    (`/Engine/EditorBlueprintResources/StandardMacros.IsValid` self
      (:`Is Valid`
        (`self.K2_DestroyActor`)))))

(fn `PlaySound`
  (`GameplayStatics.PlaySound2D` (select `/Game/Blueprints/Data/e_PickupType` (`self.PickupType`) :`NewEnumerator0` "/Game/Audio/SW_DotCollected.SW_DotCollected" :`NewEnumerator1` "/Game/Audio/SW_PowerPickup.SW_PowerPickup" :!type "SoundBase Object Reference") 0.5 1.0 0.0 null null))

(fn `UserConstructionScript`
  (`parent.UserConstructionScript`)
  (switch `/Game/Blueprints/Data/e_PickupType` (`self.PickupType`)
    (:`NewEnumerator1`
      (`SceneComponent.SetWorldScale3D` (`self.StaticMesh`) (0.5 0.5 0.5)))))