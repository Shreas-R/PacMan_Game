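; Arcade game state that tracks pickup collection and enemies for a level and drives its win and lose flow.
; On BeginPlay it gathers all pickups and enemies and creates the HUD; collecting every pickup completes the level.
; Level end and player death stop the timer and enemies, slow time, and show completion or game-over widgets.
; Power pickups make all enemies vulnerable, using a retriggerable delay so repeat pickups restart the window.
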(event `self.ReceiveBeginPlay`
  (`self.GetAllPickups`)
  (`self.CreatePlayerHUD`)
  (`self.GetAllEnemies`))

(event `/Game/Blueprints/GameFramework/Interfaces/BPI_GameFramework.IncreaseCollectedCount`
  (bind _result (`/Engine/EditorBlueprintResources/StandardMacros.IncrementInt` (`self.CollectedPickups`))
    (:`  `
      (`/Game/Blueprints/Widgets/W_UI.UpdateCurrentPickupsAndText` (`self.HUD`) _result)
      (if (>= (`self.CollectedPickups`) (`self.TotalPickups`))
        (`self.LevelEnd`)
        (message `/Game/Blueprints/GameFramework/Interfaces/BPI_GameFramework.LevelEnd` (`GameplayStatics.GetPlayerCharacter` 0))))))

(event `/Game/Blueprints/GameFramework/Interfaces/BPI_GameFramework.DebugLevelCompleted`
  (`/Game/Blueprints/Widgets/W_UI.EndTimer` (`self.HUD`) false)
  (message `/Game/Blueprints/GameFramework/Interfaces/BPI_GameFramework.LevelEnd` (`GameplayStatics.GetPlayerCharacter` 0) :!label _label)
  (`self.EndEnemyMovement`)
  (`GameplayStatics.SetGlobalTimeDilation` 0.3)
  (`KismetSystemLibrary.Delay` 0.2)
  (bind _return (message `/Game/Blueprints/GameFramework/Interfaces/BPI_GameFramework.IsFinalLevel?` (`GameplayStatics.GetGameInstance`)))
  (if _return
    (bind _returnvalue (`|CreateWidget` "/Game/Blueprints/Widgets/W_GameCompleted.W_GameCompleted_C"))
    (`UserWidget.AddToViewport` _returnvalue 9)
    (else
      (bind _returnvalue_2 (`|CreateWidget` "/Game/Blueprints/Widgets/W_LevelCompleted.W_LevelCompleted_C"))
      (`UserWidget.AddToViewport` _returnvalue_2 9))))

(event `/Game/Blueprints/GameFramework/Interfaces/BPI_GameFramework.LevelEnd`
  (`/Game/Blueprints/Widgets/W_UI.EndTimer` (`self.HUD`) true)
  (goto _label))

(event `/Game/Blueprints/GameFramework/Interfaces/BPI_GameFramework.PlayerDied`
  (`/Game/Blueprints/Widgets/W_UI.EndTimer` (`self.HUD`) false)
  (`GameplayStatics.SetGlobalTimeDilation` 0.3)
  (`KismetSystemLibrary.Delay` 0.2)
  (`self.EndEnemyMovement`)
  (bind _returnvalue (`|CreateWidget` "/Game/Blueprints/Widgets/W_GameOver.W_GameOver_C"))
  (`UserWidget.AddToViewport` _returnvalue 9))

(event `/Game/Blueprints/GameFramework/Interfaces/BPI_GameFramework.CollectedPowerPickup`
  (for _array_element (`self.EnemiesList`)
    (`/Game/Blueprints/Characters/CharacterEnemy/BP_Base_Enemy.VulnerableState` _array_element))
  (`KismetSystemLibrary.RetriggerableDelay` (`self.EnemyVulnerableDuration`))
  (for _array_element_2 (`self.EnemiesList`)
    (`/Game/Blueprints/Characters/CharacterEnemy/BP_Base_Enemy.EndVulnerableState` _array_element_2)))

(fn `CreatePlayerHUD`
  (bind _returnvalue (`|CreateWidget` "/Game/Blueprints/Widgets/W_UI.W_UI_C"))
  (bind _output_get (set `self.HUD` _returnvalue))
  (`/Game/Blueprints/Widgets/W_UI.InitializeHUD` _output_get (`self.TotalPickups`))
  (`UserWidget.AddToViewport` _output_get 0))

(fn `EndEnemyMovement`
  (for _array_element (`self.EnemiesList`)
    (`self.SetActorTickEnabled` _array_element false)
    (`MovementComponent.StopMovementImmediately` (`Character.CharacterMovement` _array_element)))
  (return))

(fn `GetAllEnemies`
  (bind _outactors (`GameplayStatics.GetAllActorsOfClass` "/Game/Blueprints/Characters/CharacterEnemy/BP_Base_Enemy.BP_Base_Enemy_C"))
  (set `self.EnemiesList` _outactors)
  (return))

(fn `GetAllPickups`
  (bind _outactors (`GameplayStatics.GetAllActorsOfClass` "/Game/Blueprints/Pickups/BP_Base_Pickup.BP_Base_Pickup_C"))
  (bind _output_get (set `self.AllCollectiblesList` _outactors))
  (set `self.TotalPickups` (`KismetArrayLibrary.Array_Length` _output_get)))

(fn `GetDifficulty`
  (returns (Difficulty :type "/Game/Blueprints/Data/e_Difficulty Enum"))
  (return "NewEnumerator0"))

(fn `GetRecordTime`
  (returns (`RecordExists?` :type Boolean) (Time :type "Float (double-precision)"))
  (return false 0.0))

(fn `IsFinalLevel?`
  (returns (Return :type Boolean))
  (return false))

(fn `IsLevelUnlocked?`
  (params (Index :type Integer))
  (returns (`Unlocked?` :type Boolean))
  (return false))

(fn `RecordNewTime`
  (params (CompletionTime :type "Float (double-precision)"))
  (returns (`NewRecord?` :type Boolean))
  (return false))

(fn `UserConstructionScript`)