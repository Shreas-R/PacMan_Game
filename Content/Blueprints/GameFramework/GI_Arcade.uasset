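; Game instance for an arcade game that owns level progression, difficulty and record times across level loads.
; It loads an SGO_Arcade save on Init and writes a fresh save object when levels unlock or completion times are recorded.
; An ordered level array drives delayed next-level or restart loading, wrapping to the first level after the last.
; A map keyed by level stores unlock state and best time, with zero meaning no record.
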(event `self.ReceiveInit`
  (`self.LoadGameSave`))

(event `/Game/Blueprints/GameFramework/Interfaces/BPI_GameFramework.OpenNextLevel`
  (params (DelayBeforeOpen :type "Float (double-precision)"))
  (`KismetSystemLibrary.Delay` DelayBeforeOpen)
  (bind _nextlevel (`self.GetNextLevel`))
  (bind _output_get (set `self.Current` _nextlevel))
  (`self.UnlockNextLevel` _output_get)
  (`GameplayStatics.OpenLevelBySoftObjectPtr` _output_get))

(event `/Game/Blueprints/GameFramework/Interfaces/BPI_GameFramework.OpenSameLevel`
  (params (DelayBeforeOpen :type "Float (double-precision)"))
  (`KismetSystemLibrary.Delay` DelayBeforeOpen)
  (`GameplayStatics.OpenLevelBySoftObjectPtr` (`self.Current`)))

(event `/Game/Blueprints/GameFramework/Interfaces/BPI_GameFramework.SetCurrentLevel`
  (params (ArrayIndex :type Integer))
  (set `self.Current` (`|GetArrayItem` (`self.GameLevels`) ArrayIndex)))

(event `/Game/Blueprints/GameFramework/Interfaces/BPI_GameFramework.SaveGame`
  (bind _savegameobject (`self.SaveGameObject`))
  (bind _returnvalue (`GameplayStatics.CreateSaveGameObject` "/Game/Blueprints/GameFramework/SGO_Arcade.SGO_Arcade_C"))
  (set `self.SaveGameObject` _returnvalue)
  (set `/Game/Blueprints/GameFramework/SGO_Arcade.SavedLevelStatuses` (`self.GameLevelStatuses`) _savegameobject)
  (set `/Game/Blueprints/GameFramework/SGO_Arcade.SavedDifficulty` (`self.GameDifficulty`) _savegameobject)
  (`GameplayStatics.SaveGameToSlot` (`self.SaveGameObject`) (`self.SaveGameSlotName`)))

(event `/Game/Blueprints/GameFramework/Interfaces/BPI_GameFramework.SetDifficulty`
  (params (Difficulty :type "/Game/Blueprints/Data/e_Difficulty Enum" :default "NewEnumerator0"))
  (set `self.GameDifficulty` Difficulty))

(fn `GetDifficulty`
  (returns (Difficulty :type "/Game/Blueprints/Data/e_Difficulty Enum"))
  (return (`self.GameDifficulty`)))

(fn `GetIndexOfNextLevel`
  (params (Index :type Integer))
  (returns (ReturnValue :type Integer))
  (return (select `bool` (>= Index (`KismetArrayLibrary.Array_LastIndex` (`self.GameLevels`))) :`false` (+ Index 1))))

(fn `GetNextLevel`
  (returns (NextLevel :type "World Soft Object Reference"))
  (for (_array_element _array_index) (`self.GameLevels`)
    (if (== _array_element (`self.Current`))
      (break)))
  (return (`|GetArrayItem` (`self.GameLevels`) (`self.GetIndexOfNextLevel` _array_index))))

(fn `GetRecordTime`
  (returns (`RecordExists?` :type Boolean) (Time :type "Float (double-precision)"))
  (bind (_value _returnvalue) (`BlueprintMapLibrary.Map_Find` (`self.GameLevelStatuses`) (`self.Current`)))
  (if _returnvalue
    (if (!= (`.RecordTime_5_DC73CD154D44C050A74D98BD8B586028` (break `/Game/Blueprints/GameFramework/s_LevelStatus` _value)) 0.0)
      (return true (`.RecordTime_5_DC73CD154D44C050A74D98BD8B586028` (break `/Game/Blueprints/GameFramework/s_LevelStatus` _value)))
      (else
        (return false 0.0)))
    (else
      (return false 0.0))))

(fn `IsFinalLevel?`
  (returns (Return :type Boolean))
  (bind _gamelevels (`self.GameLevels`))
  (return (== (`|GetArrayItem` _gamelevels (`KismetArrayLibrary.Array_LastIndex` _gamelevels)) (`self.Current`))))

(fn `IsLevelUnlocked?`
  (params (Index :type Integer))
  (returns (`Unlocked?` :type Boolean))
  (return (break `/Game/Blueprints/GameFramework/s_LevelStatus` (`BlueprintMapLibrary.Map_Find` (`self.GameLevelStatuses`) (`|GetArrayItem` (`self.GameLevels`) Index)))))

(fn `LoadGameSave`
  (bind _returnvalue (`GameplayStatics.LoadGameFromSlot` (`self.SaveGameSlotName`)))
  (bind _assgo_von_darcade (cast `/Game/Blueprints/GameFramework/SGO_Arcade` _returnvalue))
  (bind _output_get (set `self.SaveGameObject` _assgo_von_darcade))
  (set `self.GameLevelStatuses` (`/Game/Blueprints/GameFramework/SGO_Arcade.SavedLevelStatuses` _output_get))
  (set `self.GameDifficulty` (`/Game/Blueprints/GameFramework/SGO_Arcade.SavedDifficulty` _output_get))
  (return))

(fn `RecordNewTime`
  (params (CompletionTime :type "Float (double-precision)"))
  (returns (`NewRecord?` :type Boolean))
  (bind (_value _returnvalue) (`BlueprintMapLibrary.Map_Find` (`self.GameLevelStatuses`) (`self.Current`)))
  (if _returnvalue
    (if (or (< CompletionTime (`.RecordTime_5_DC73CD154D44C050A74D98BD8B586028` (break `/Game/Blueprints/GameFramework/s_LevelStatus` _value))) (== (`.RecordTime_5_DC73CD154D44C050A74D98BD8B586028` (break `/Game/Blueprints/GameFramework/s_LevelStatus` _value)) 0.0))
      _
      (else
        (`self.SaveGame`)
        (return false))))
  (`BlueprintMapLibrary.Map_Add` (`self.GameLevelStatuses`) (`self.Current`) (make `/Game/Blueprints/GameFramework/s_LevelStatus` true CompletionTime))
  (`self.SaveGame`)
  (return true))

(fn `UnlockNextLevel`
  (params (Level :type "World Soft Object Reference (by ref)"))
  (bind _gamelevelstatuses (`self.GameLevelStatuses`))
  (bind (_value _returnvalue) (`BlueprintMapLibrary.Map_Find` _gamelevelstatuses Level))
  (if _returnvalue
    (if (not (break `/Game/Blueprints/GameFramework/s_LevelStatus` _value))
      (`BlueprintMapLibrary.Map_Add` _gamelevelstatuses Level (make `/Game/Blueprints/GameFramework/s_LevelStatus` true (`.RecordTime_5_DC73CD154D44C050A74D98BD8B586028` (break `/Game/Blueprints/GameFramework/s_LevelStatus` _value))))
      (`self.SaveGame`))
    (return)
    (else
      (return))))