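; Base player character that handles movement speed, death and level end, with camera distance and height set by the game instance's difficulty.
; Death notifies the game state, plays a sound and runs LevelEnd, which disables movement and tints the character white if alive, otherwise the enemy's color or black.
; Construction applies default walk and jump speeds.
; The 0 key triggers a debug level-complete message; difficulty, record and unlock functions return placeholder values.
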(event `self.ReceiveBeginPlay`
  (bind _returnvalue (`GameplayStatics.GetPlayerController` 0))
  (`WidgetBlueprintLibrary.SetInputMode_GameOnly` _returnvalue)
  (set `PlayerController.bShowMouseCursor` false _returnvalue)
  (`self.UpdateCameraBoomLocation`))

(event `self.CharacterDeath`
  (if (`self.CanCharacterDie?`)
    (set `self.IsCharacterAlive?` false)
    (set `self.CanCharacterDie?` false)
    (message `/Game/Blueprints/GameFramework/Interfaces/BPI_GameFramework.PlayerDied` (`GameplayStatics.GetGameState`))
    (`self.LevelEnd`)
    (`GameplayStatics.PlaySound2D` "/Game/Audio/SW_HeroDeath.SW_HeroDeath" 1.0 1.0 0.0 null null)))

(event `/Game/Blueprints/GameFramework/Interfaces/BPI_GameFramework.LevelEnd`
  (`self.DisableInteraction`)
  (`self.ChangeColors` (`self.SelectColorToChangeTo`) 0.1))

(event `Key|Zero`
  (params (Key :type "Key Structure"))
  (:`Pressed`
    (message `/Game/Blueprints/GameFramework/Interfaces/BPI_GameFramework.DebugLevelCompleted` (`GameplayStatics.GetGameState`))))

(fn `ChangeMaxSpeed`
  (params (MaxWalkSpeed :type "Float (double-precision)") (JumpZVelocity :type "Float (double-precision)"))
  (bind _charactermovement (`self.CharacterMovement`))
  (set `CharacterMovementComponent.MaxWalkSpeed` MaxWalkSpeed _charactermovement)
  (set `CharacterMovementComponent.JumpZVelocity` JumpZVelocity _charactermovement))

(fn `DisableInteraction`
  (set `self.CanCharacterDie?` false)
  (`CharacterMovementComponent.DisableMovement` (`self.CharacterMovement`)))

(fn `GetDifficulty`
  (returns (Difficulty :type "/Game/Blueprints/Data/e_Difficulty Enum"))
  (return "NewEnumerator0"))

(fn `GetRecordTime`
  (returns (`RecordExists?` :type Boolean) (Time :type "Float (double-precision)"))
  (return false 0.0))

(fn `IsFinalLevel?`
  (returns (Return :type Boolean))
  (return false))

(fn `IsLevelUnlocked?`
  (params (Index :type Integer))
  (returns (`Unlocked?` :type Boolean))
  (return false))

(fn `RecordNewTime`
  (params (CompletionTime :type "Float (double-precision)"))
  (returns (`NewRecord?` :type Boolean))
  (return false))

(fn `SelectColorToChangeTo`
  (returns (ReturnValue :type "LinearColor Structure"))
  (bind _enemy (`self.Enemy`))
  (return (select `bool` (`self.IsCharacterAlive?`) :`false` (select `bool` (`KismetSystemLibrary.IsValid` _enemy) :`false` (struct :`A` 1.0) :`true` (`/Game/Blueprints/Characters/BP_Master_Character.Color` _enemy)) :`true` (struct :`R` 1.0 :`G` 1.0 :`B` 1.0 :`A` 1.0))))

(fn `UpdateCameraBoomLocation`
  (bind _cameraboom (`self.CameraBoom`))
  (bind _difficulty (message `/Game/Blueprints/GameFramework/Interfaces/BPI_GameFramework.GetDifficulty` (`GameplayStatics.GetGameInstance`)))
  (set `SpringArmComponent.TargetArmLength` (select `/Game/Blueprints/Data/e_Difficulty` _difficulty :`NewEnumerator0` 500.0 :`NewEnumerator1` 300.0 :`NewEnumerator2` 120.0 :!type "Float (single-precision)") _cameraboom)
  (set `SpringArmComponent.TargetOffset` (`KismetMathLibrary.MakeVector` 0.0 0.0 (select `/Game/Blueprints/Data/e_Difficulty` _difficulty :`NewEnumerator0` 200.0 :`NewEnumerator1` 100.0 :`NewEnumerator2` 60.0)) _cameraboom)
  (return))

(fn `UserConstructionScript`
  (bind (_defaultwalkspeedandjump_x _defaultwalkspeedandjump_y) (`KismetMathLibrary.BreakVector2D` (`self.DefaultWalkSpeedAndJump`)))
  (`parent.UserConstructionScript`)
  (`self.ChangeMaxSpeed` _defaultwalkspeedandjump_x _defaultwalkspeedandjump_y))