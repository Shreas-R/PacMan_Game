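; Base enemy character with Pac-Man-style ghost behavior: it chases the player, flees when vulnerable, returns home when killed, then recovers.
; Tick switches on a behavior enum, driving simple move-to for chase and return, and throttled random-point AI moves for fleeing.
; Collision overlap kills either enemy or player depending on vulnerability.
; State events adjust behavior and color; death also slows walk speed until the enemy reaches base.
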(event `self.ReceiveBeginPlay`
  (set `self.EnemyController` (`self.GetController`))
  (`self.GetPlayerCharacter`
    (:`Success`
      (`KismetSystemLibrary.Delay` (`self.ChaseDelay`))
      (`self.SetActorTickEnabled` true))))

(event `self.ReceiveTick`
  (params (DeltaSeconds :type "Float (single-precision)"))
  (switch `/Game/Blueprints/Data/e_EnemyBehavior` (`self.CurrentEnemyBehavior`)
    (:`NewEnumerator1`
      (`AIBlueprintHelperLibrary.SimpleMoveToActor` (`self.EnemyController`) (`self.PlayerCharacter`)))
    (:`NewEnumerator0`
      (`/Engine/EditorBlueprintResources/StandardMacros.DoOnce` false :!label _label
        (:`Completed`
          (`|AIMoveTo` self (`NavigationSystemV1.K2_GetRandomReachablePointInRadius` (`self.K2_GetActorLocation` (`self.PlayerCharacter`)) 10000.0 null null) null 100.0
            (:`then`
              _)
            (:`OnSuccess`
              _)
            (:`OnFail`
              _))
          (`KismetSystemLibrary.Delay` (`KismetMathLibrary.RandomFloatInRange` 0.5 2.0))
          (goto _label :!via `Reset`))))
    (:`NewEnumerator2`
      (if (== (`self.K2_GetActorLocation`) (`self.K2_GetActorLocation` (`self.HomeBase`)) :`ErrorTolerance` 100.0)
        (set `self.CurrentEnemyBehavior` "NewEnumerator3")
        (set `CharacterMovementComponent.MaxWalkSpeed` (`self.MaxWalkSpeed`) (`self.CharacterMovement`))
        (else
          (`AIBlueprintHelperLibrary.SimpleMoveToActor` (`self.EnemyController`) (`self.HomeBase`)))))
    (:`NewEnumerator3`
      (`KismetSystemLibrary.Delay` (`self.RestDelay`))
      (`self.ReturnToNormal`))))

(event `self.CollisionRadius.OnComponentBeginOverlap`
  (params (OverlappedComponent :type "PrimitiveComponent Object Reference") (OtherActor :type "Actor Object Reference") (OtherComp :type "PrimitiveComponent Object Reference") (OtherBodyIndex :type Integer) (bFromSweep :type Boolean) (SweepResult :type "HitResult Structure (by ref)"))
  (if (== (`self.PlayerCharacter`) OtherActor)
    (if (`self.CanCharacterDie?`)
      (`self.CharacterDeath`)
      (else
        (`self.KillPlayer`)))))

(event `self.CharacterDeath`
  (set `self.CurrentEnemyBehavior` "NewEnumerator2")
  (set `self.IsCharacterAlive?` false)
  (set `CharacterMovementComponent.MaxWalkSpeed` 250.0 (`self.CharacterMovement`))
  (`self.ChangeColors` (struct :`R` 0.019608 :`G` 0.019608 :`B` 0.835294 :`A` 1.0) 0.2))

(event `ReturnToNormal`
  (`self.KillPlayerIfOverlapping`)
  (set `self.CurrentEnemyBehavior` "NewEnumerator1")
  (set `self.IsCharacterAlive?` true)
  (set `self.CanCharacterDie?` false)
  (`self.ChangeColors` (`self.Color`) 0.2))

(event `VulnerableState`
  (if (`self.IsCharacterAlive?`)
    (set `self.CurrentEnemyBehavior` "NewEnumerator0")
    (set `self.CanCharacterDie?` true)
    (`self.ChangeColors` (struct :`R` 1.0 :`G` 1.0 :`B` 1.0 :`A` 1.0) 0.2)))

(event `EndVulnerableState`
  (if (`self.IsCharacterAlive?`)
    (`self.ReturnToNormal`)))

(fn `KillPlayer`
  (bind _playercharacter (`self.PlayerCharacter`))
  (if (`/Game/Blueprints/Characters/BP_Master_Character.CanCharacterDie?` _playercharacter)
    (set `/Game/Blueprints/Characters/CharacterPlayer/BP_Base_PlayerCharacter.Enemy` self _playercharacter)
    (`self.CharacterDeath` _playercharacter))
  (return))

(fn `KillPlayerIfOverlapping`
  (if (`PrimitiveComponent.IsOverlappingActor` (`self.CollisionRadius`) (`self.PlayerCharacter`))
    (`self.KillPlayer`)
    (return)
    (else
      (return))))

(fn `UserConstructionScript`
  (`parent.UserConstructionScript`)
  (set `CharacterMovementComponent.MaxWalkSpeed` (`self.MaxWalkSpeed`) (`self.CharacterMovement`)))